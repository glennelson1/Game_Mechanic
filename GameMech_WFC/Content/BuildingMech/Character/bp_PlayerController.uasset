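; Player controller for grid-based building placement, active from BeginPlay, with the building type set by placement info updates.
; A preview actor spawns in placement mode and snaps each tick to the closest MyGridManager position.
; Left click spawns the building at the preview, marks its grid cell occupied and registers only BB_Building1 types with Bp_BuildingManager.
; Placement updates replace the preview, except one enum mode, which disables placement.
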(event `self.ReceiveBeginPlay`
  (`self.SetPlacementModeEnabled` true))

(event `self.ReceiveTick`
  (params (DeltaSeconds :type "Float (single-precision)"))
  (if (`self.PlacementModeEnabled`)
    (`self.UpdatePlacement_0`)))

(event `Key|LeftMouseButton`
  (params (Key :type "Key Structure"))
  (:`Pressed`
    (if (`self.PlacementModeEnabled`)
      (`self.SpawnBuilding1`))))

(event `OnPlacmentInfoUpdated`
  (params (InPlaceableActorType :type "/Game/BuildingMech/Buildings/BP_BaseBuilding Class Reference") (InPlaceableMode :type "/Game/BuildingMech/Buildings/BuildingTypeEnum Enum" :default "NewEnumerator3"))
  (bind _placeableactor (`self.PlaceableActor`))
  (set `self.PlaceableActorType` InPlaceableActorType)
  (bind _output_get (set `self.PlaceeableBuildingType` InPlaceableMode))
  (if (`|EnumEquality` _output_get "NewEnumerator3")
    (`self.SetPlacementModeEnabled` false)
    (else
      (`/Engine/EditorBlueprintResources/StandardMacros.IsValid` _placeableactor
        (:`Is Valid`
          (`self.K2_DestroyActor` _placeableactor))
        (:`Is Not Valid`
          _))
      (`self.RefreshPlaceableBuilding`))))

(fn `RefreshPlaceableBuilding`
  (bind _returnvalue (`|SpawnActorFromClass` (`self.PlaceableActorType`) (`KismetMathLibrary.MakeTransform` (0.0 0.0 -10000.0)) "AlwaysSpawn" "OverrideRootScale" null null))
  (bind _asbp_base_building (cast `/Game/BuildingMech/Buildings/BP_BaseBuilding` _returnvalue)
    (:`then`
      (bind _output_get (set `self.PlaceableActor` _asbp_base_building))
      (bind _returnvalue_2 (`self.GetComponentByClass` _output_get "/Game/BuildingMech/Buildings/ClickableComp.ClickableComp_C"))
      (`/Engine/EditorBlueprintResources/StandardMacros.IsValid` _returnvalue_2
        (:`Is Valid`
          (`/Game/BuildingMech/Buildings/ClickableComp.InPlacementMode` _returnvalue_2))))
    (:`CastFailed`
      (`AutomationBlueprintFunctionLibrary.AddExpectedLogError` "Error"))))

(fn `SetPlacementModeEnabled`
  (params (IsEnabled :type Boolean))
  (bind _placeableactor (`self.PlaceableActor`))
  (if (== IsEnabled (`self.PlacementModeEnabled`))
    (return)
    (else
      (bind _output_get (set `self.PlacementModeEnabled` IsEnabled))
      (if _output_get
        (`self.RefreshPlaceableBuilding`)
        (else
          (`/Engine/EditorBlueprintResources/StandardMacros.IsValid` _placeableactor
            (:`Is Valid`
              (`self.K2_DestroyActor` _placeableactor))))))))

(fn `SpawnBuilding1`
  (bind _placeableactor (`self.PlaceableActor`))
  (bind _returnvalue (`|SpawnActorFromClass` (`self.PlaceableActorType`) (`self.GetTransform` _placeableactor) "AlwaysSpawn" "OverrideRootScale" null null))
  (bind _returnvalue_2 (`GameplayStatics.GetActorOfClass` "/Game/BuildingMech/Grid/MyGridManager.MyGridManager_C"))
  (bind _outputvector (`/Game/BuildingMech/Grid/MyGridManager.GetClosestGridCell` _returnvalue_2 (`self.K2_GetActorLocation` _placeableactor)))
  (bind _asbp_grid_actor (cast `/Game/BuildingMech/Grid/bp_GridActor` _outputvector))
  (bind _asbp_base_building (cast `/Game/BuildingMech/Buildings/BP_BaseBuilding` _returnvalue))
  (`/Game/BuildingMech/Grid/bp_GridActor.SetOccupied` _asbp_grid_actor (`/Game/BuildingMech/Buildings/BP_BaseBuilding.BuildingType` _asbp_base_building) _returnvalue)
  (set `/Game/BuildingMech/Buildings/BP_BaseBuilding.GridCellRef` _asbp_grid_actor _asbp_base_building)
  ;[1 1 1] Notify manager of new building
  (bind _asbb_building_1 (cast `/Game/BuildingMech/Buildings/BB_Building1` _returnvalue))
  (bind _returnvalue_3 (`GameplayStatics.GetActorOfClass` "/Game/BuildingMech/Buildings/Bp_BuildingManager.Bp_BuildingManager_C"))
  (`/Game/BuildingMech/Buildings/Bp_BuildingManager.AddBuilding` _returnvalue_3 _asbb_building_1))

(fn `UpdatePlacement_0`
  (bind _returnvalue (`self.UpdatePlacement` (0.0 0.0 0.0)))
  (bind _returnvalue_2 (`GameplayStatics.GetActorOfClass` "/Game/BuildingMech/Grid/MyGridManager.MyGridManager_C"))
  (bind _outputvector (`/Game/BuildingMech/Grid/MyGridManager.GetClosestGridPosition` _returnvalue_2 _returnvalue))
  (`self.K2_SetActorLocation` (`self.PlaceableActor`) _outputvector false false))

(fn `UserConstructionScript`)