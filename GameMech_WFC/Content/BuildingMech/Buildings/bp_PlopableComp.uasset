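; Actor component for placeable buildings that shows whether the owner's current location is a valid placement spot.
; On BeginPlay and every Tick it finds the MyGridManager, gets the grid cell closest to the owner, and marks placement valid if that cell is unoccupied.
; It then sets the first material slot of all the owner's static meshes to the valid or invalid placement material.
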(event `self.ReceiveBeginPlay`
  (`self.UpdateState`))

(event `self.ReceiveTick`
  (params (DeltaSeconds :type "Float (single-precision)"))
  (`self.UpdateState`))

(fn `UpdateState`
  (locals (NewLocalVar_0 :type "Object Object Reference"))
  (bind _returnvalue (`GameplayStatics.GetActorOfClass` "/Game/BuildingMech/Grid/MyGridManager.MyGridManager_C"))
  (bind _outputvector (`/Game/BuildingMech/Grid/MyGridManager.GetClosestGridCell` _returnvalue (`Actor.K2_GetActorLocation` (`self.GetOwner`))))
  (bind _output_get (set `self.IsPlacementVaild` (not (`GridActor.m_IsOccupied` _outputvector))))
  (for _array_element (`Actor.K2_GetComponentsByClass` (`self.GetOwner`) "/Script/Engine.StaticMeshComponent")
    (if _output_get
      (`PrimitiveComponent.SetMaterial` _array_element 0 (`self.PloppableMaterial`))
      (else
        (`PrimitiveComponent.SetMaterial` _array_element 0 (`self.InvaildPloppablematerial`))))))