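; BP_Grid is a grid actor, apparently for drawing lines and a selectable tile, still mostly scaffolding.
; Its construction script creates two dynamic instances of M_Grid through CreateMaterialInstance, setting colour and opacity separately for lines and selection.
; Line creation, grid sizing, location-to-tile conversion, selection and validity checks are empty stubs or return default values, so no geometry is built.
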(fn `CreateLine`
  (params (Start :type "Vector Structure") (End :type "Vector Structure") (Thickness :type "Float (double-precision)") (Vertices :type "Array of Vector Structure") (Triangles :type "Array of Integer")))

(fn `CreateMaterialInstance`
  (params (Colour :type "LinearColor Structure") (Opacity :type "Float (double-precision)"))
  (returns (`Material Instance` :type "MaterialInstanceDynamic Object Reference"))
  (bind _returnvalue (`KismetMaterialLibrary.CreateDynamicMaterialInstance` "/Game/Grid/Test1/M_Grid.M_Grid"))
  (`MaterialInstanceDynamic.SetVectorParameterValue` _returnvalue "Colour" Colour)
  (`MaterialInstanceDynamic.SetScalarParameterValue` _returnvalue "Opacity" Opacity)
  (return _returnvalue))

(fn `GridHeight`)

(fn `GridWidth`)

(fn `LocationToTiles`
  (params (Location :type "Vector Structure"))
  (returns (IsVaild :type Boolean) (Row :type Integer) (Column :type Integer))
  (return false 0 0))

(fn `SetSelectedTile`
  (params (Row :type Integer) (Column :type Integer)))

(fn `TileToGridLocation`
  (params (Row :type Integer) (Column :type Integer) (IsCentre :type Integer))
  (returns (IsValid :type Boolean) (GridLocation :type "Vector2D Structure"))
  (return false (0.0 0.0)))

(fn `UserConstructionScript`
  (locals (LineMaterialInstance :type "MaterialInstanceDynamic Object Reference") (SelectionSelectionInstance :type "MaterialInstanceDynamic Object Reference"))
  (bind _material_instance (`self.CreateMaterialInstance` (`self.LineColour`) (`self.LineOpacity`)))
  (set `local.LineMaterialInstance` _material_instance)
  (bind _material_instance_2 (`self.CreateMaterialInstance` (`self.SelectionColour`) (`self.SelectionOpacity`)))
  (set `local.SelectionSelectionInstance` _material_instance_2))