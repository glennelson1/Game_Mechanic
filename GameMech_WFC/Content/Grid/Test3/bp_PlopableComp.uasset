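; Placement-feedback component that shows whether its owning actor sits over a free grid cell.
; On BeginPlay and every Tick, it looks up Bp_GridManager with GetActorOfClass and queries the closest cell to the owner's location.
; It sets IsPlacementVaild from that cell's occupancy, then swaps material slot 0 on all the owner's static meshes between the valid and invalid ploppable materials.
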(event `self.ReceiveBeginPlay`
  (`self.UpdateState`))

(event `self.ReceiveTick`
  (params (DeltaSeconds :type "Float (single-precision)"))
  (`self.UpdateState`))

(fn `UpdateState`
  (locals (NewLocalVar_0 :type "/Game/Grid/Test3/GameObjects/bp_GridCell Object Reference"))
  (bind _returnvalue (`GameplayStatics.GetActorOfClass` "/Game/Grid/Test3/bp_GridManager.bp_GridManager_C"))
  (bind _outputvector (`/Game/Grid/Test3/bp_GridManager.GetClosestGridCell` _returnvalue (`Actor.K2_GetActorLocation` (`self.GetOwner`))))
  (bind _output_get (set `self.IsPlacementVaild` (not (`/Game/Grid/Test3/GameObjects/bp_GridCell.IsOccupied` _outputvector))))
  (for _array_element (`Actor.K2_GetComponentsByClass` (`self.GetOwner`) "/Script/Engine.StaticMeshComponent")
    (if _output_get
      (`PrimitiveComponent.SetMaterial` _array_element 0 (`self.PloppableMaterial`))
      (else
        (`PrimitiveComponent.SetMaterial` _array_element 0 (`self.InvaildPloppablematerial`))))))