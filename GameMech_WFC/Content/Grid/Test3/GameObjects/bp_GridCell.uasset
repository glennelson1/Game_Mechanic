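; Grid cell actor that records whether it is occupied, by which building type and by which actor.
; SetOccupied sets that state from the building type and actor passed in.
; DebugShowNeighbourOccupied turns the cell's sphere red as a debug marker.
; The cell references north, east, west and south neighbours, but the calls that would trigger their debug highlight are unconnected and never run.
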(event `SetOccupied`
  (params (NewBuildingType :type "/Game/Grid/Test3/GameObjects/BuildingTypeEnum Enum" :default "NewEnumerator3") (OccupingActorRef :type "Actor Object Reference"))
  (set `self.IsOccupied` true)
  (set `self.OccupingType` NewBuildingType)
  (set `self.OccupingActor` OccupingActorRef))

(event `DebugShowNeighbourOccupied`
  (`PrimitiveComponent.SetMaterial` (`self.Sphere`) 0 "/Game/Grid/Materials/m_red.m_red"))

(fn `UserConstructionScript`)