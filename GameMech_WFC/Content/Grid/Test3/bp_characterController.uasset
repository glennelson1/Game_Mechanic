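; Controller for grid-based building placement, with placement mode switched on at BeginPlay.
; Enabling the mode spawns a preview of PlaceableActorType, which follows a mouse trace each Tick, snapped to Bp_GridManager's closest grid position.
; Left click spawns a building there if the preview's Bp_PlopableComp reports valid placement.
; The new building occupies and references its grid cell, and BB_Building1 types also register with Bp_BuildingManager.
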(event `self.ReceiveBeginPlay`
  (`self.SetPlacementModeEnabled` true))

(event `self.ReceiveTick`
  (params (DeltaSeconds :type "Float (single-precision)"))
  (if (`self.PlacementModeEnabled`)
    (`self.UpdatePlacement`)))

(event `Key|LeftMouseButton`
  (params (Key :type "Key Structure"))
  (:`Pressed`
    (if (`self.PlacementModeEnabled`)
      (`self.SpawnBuilding`))))

(fn `SetPlacementModeEnabled`
  (params (IsEnabled :type Boolean))
  (bind _placeableactor (`self.PlaceableActor`))
  (if (== IsEnabled (`self.PlacementModeEnabled`))
    (return)
    (else
      (bind _output_get (set `self.PlacementModeEnabled` IsEnabled))
      (if _output_get
        (bind _returnvalue (`|SpawnActorFromClass` (`self.PlaceableActorType`) (`KismetMathLibrary.MakeTransform` (0.0 0.0 -10000.0)) "AlwaysSpawn" "OverrideRootScale" null null))
        (bind _asbp_base_building (cast `/Game/Grid/Test3/GameObjects/BP_BaseBuilding` _returnvalue)
          (:`then`
            (bind _output_get_2 (set `self.PlaceableActor` _asbp_base_building))
            (bind _returnvalue_2 (`self.GetComponentByClass` _output_get_2 "/Game/Grid/Test3/ClickableComp.ClickableComp_C"))
            (`/Engine/EditorBlueprintResources/StandardMacros.IsValid` _returnvalue_2
              (:`Is Valid`
                (`/Game/Grid/Test3/ClickableComp.InPlacementMode` _returnvalue_2))
              (:`Is Not Valid`
                _))
            (`AddComponent|NODE_Addbp_PlopableComp-0` :`self` _asbp_base_building))
          (:`CastFailed`
            (`AutomationBlueprintFunctionLibrary.AddExpectedLogError` "Error")))
        (else
          (`/Engine/EditorBlueprintResources/StandardMacros.IsValid` _placeableactor
            (:`Is Valid`
              (`self.K2_DestroyActor` _placeableactor))))))))

(fn `SpawnBuilding`
  (bind _placeableactor (`self.PlaceableActor`))
  (bind _returnvalue (`self.GetComponentByClass` (`self.PlaceableActor`) "/Game/Grid/Test3/bp_PlopableComp.bp_PlopableComp_C"))
  (`/Engine/EditorBlueprintResources/StandardMacros.IsValid` _returnvalue
    (:`Is Valid`
      (if (`/Game/Grid/Test3/bp_PlopableComp.IsPlaceMentVaild` _returnvalue)
        (bind _returnvalue_2 (`|SpawnActorFromClass` (`self.PlaceableActorType`) (`self.GetTransform` _placeableactor) "AlwaysSpawn" "OverrideRootScale" null null))
        (bind _returnvalue_3 (`GameplayStatics.GetActorOfClass` "/Game/Grid/Test3/bp_GridManager.bp_GridManager_C"))
        (bind _outputvector (`/Game/Grid/Test3/bp_GridManager.GetClosestGridCell` _returnvalue_3 (`self.K2_GetActorLocation` _placeableactor)))
        (bind _asbp_base_building (cast `/Game/Grid/Test3/GameObjects/BP_BaseBuilding` _returnvalue_2))
        (`/Game/Grid/Test3/GameObjects/bp_GridCell.SetOccupied` _outputvector (`/Game/Grid/Test3/GameObjects/BP_BaseBuilding.BuildingType` _asbp_base_building) _returnvalue_2)
        (set `/Game/Grid/Test3/GameObjects/BP_BaseBuilding.GridCellRef` _outputvector _asbp_base_building)
        ;[1 1 1] Notify manager of new building
        (bind _asbb_building_1 (cast `/Game/Grid/Test3/GameObjects/BB_Building1` _returnvalue_2))
        (bind _returnvalue_4 (`GameplayStatics.GetActorOfClass` "/Game/Grid/Test3/Buildings/Bp_BuildingManager.Bp_BuildingManager_C"))
        (`/Game/Grid/Test3/Buildings/Bp_BuildingManager.AddBuilding` _returnvalue_4 _asbb_building_1)))))

(fn `UpdatePlacement`
  (bind (_worldlocation _worlddirection) (`self.DeprojectMousePositionToWorld`))
  (bind _outhit (`KismetSystemLibrary.LineTraceSingle` _worldlocation (+ _worlddirection (* _worlddirection 100000.0)) "TraceTypeQuery4"))
  (bind (_bblockinghit _binitialoverlap _time _distance _location) (`GameplayStatics.BreakHitResult` _outhit))
  (if _bblockinghit
    (bind _returnvalue (`GameplayStatics.GetActorOfClass` "/Game/Grid/Test3/bp_GridManager.bp_GridManager_C"))
    (bind _outputvector (`/Game/Grid/Test3/bp_GridManager.GetClosestGridPosition` _returnvalue _location))
    (`self.K2_SetActorLocation` (`self.PlaceableActor`) _outputvector false false)))

(fn `UserConstructionScript`)